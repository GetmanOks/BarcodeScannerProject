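; Controller Blueprint that drives a barcode scanner through Enhanced Input and a UI widget.
; On BeginPlay it shows the cursor, switches to Game and UI input, adds the scanner mapping context and puts the scanner widget on screen.
; It caches the first BP_BarcodeScannerActor in the level, and start and stop input actions forward to that actor, printing a message if it is invalid.
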(event Input|EnhancedActionEvents|EnhancedInputActionIA_StartScanner
  (params (ActionValue :type Boolean) (ElapsedSeconds :type Float%20%28double-precision%29) (TriggeredSeconds :type Float%20%28double-precision%29) (InputAction :type Input%20Action%20Object%20Reference :default "/Game/Input/IA_StartScanner.IA_StartScanner"))
  (bind _scanneractor (Variables|Default|GetScannerActor)
    (:then
      (Default|StartScanner _scanneractor))
    (:else
      (Development|PrintString "No scanner actor found"))))

(event Input|EnhancedActionEvents|EnhancedInputActionIA_StopScanner
  (params (ActionValue :type Boolean) (ElapsedSeconds :type Float%20%28double-precision%29) (TriggeredSeconds :type Float%20%28double-precision%29) (InputAction :type Input%20Action%20Object%20Reference :default "/Game/Input/IA_StopScanner.IA_StopScanner"))
  (bind _scanneractor (Variables|Default|GetScannerActor)
    (:then
      (Default|StopScanner _scanneractor))
    (:else
      (Development|PrintString "No scanner actor found"))))

(event EventBeginPlay
  (bind _returnvalue (Game|GetPlayerController 0))
  (Variables|/Script/Engine.PlayerController|SetbShowMouseCursor _returnvalue true)
  (Input|SetInputModeGameandUI _returnvalue 0 "DoNotLock" false true)
  (Input|AddMappingContext (PlayerController|LocalPlayerSubsystems|GetEnhancedInputLocalPlayerSubsystem _returnvalue) (Variables|Default|GetIMC_BarcodeScanner) 0 "(bIgnoreAllPressedKeysUntilRelease=True,bForceImmediately=False,bNotifyUserSettings=False)")
  (bind _returnvalue_2 (UserInterface|CreateWidget "/Game/UI/WBP_BarcodeScannerWidget.WBP_BarcodeScannerWidget_C"))
  (bind _output_get (Variables|Default|SetScannerWidget _returnvalue_2))
  (UserInterface|Viewport|AddtoViewport _output_get 0)
  (bind _outactors (Actor|GetAllActorsOfClass "/Game/Blueprints/BP_BarcodeScannerActor.BP_BarcodeScannerActor_C"))
  (Variables|Default|SetScannerActor (Utilities|Array|Get(acopy) _outactors)))

(fn ConstructionScript)