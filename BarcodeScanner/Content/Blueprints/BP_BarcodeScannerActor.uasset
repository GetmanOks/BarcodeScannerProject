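; BP_BarcodeScannerActor is an actor that holds the state of a barcode scanner: active flag, status message and last scanned code.
; BeginPlay sets it inactive and ready, while StartScanner and StopScanner toggle the flag, update the status and print a message.
; OnBarcodeScanned stores the passed code and shows it in the status without checking the active flag.
; It contains no detection logic and no calls to these functions.
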(event EventBeginPlay
  (Variables|Default|SetIsScannerActive false)
  (Variables|Default|SetScannerStatus "Scanner is ready")
  (Development|PrintString "Scanner initialized"))

(event Collision|EventActorBeginOverlap
  (params (OtherActor :type Actor%20Object%20Reference)))

(event EventTick
  (params (DeltaSeconds :type Float%20%28single-precision%29)))

(fn ConstructionScript)

(fn StartScanner
  (Variables|Default|SetIsScannerActive true)
  (Variables|Default|SetScannerStatus "Scanner is active")
  (Development|PrintString "Scanner started"))

(fn StopScanner
  (Variables|Default|SetIsScannerActive false)
  (Variables|Default|SetScannerStatus "Scanner is stopped")
  (Development|PrintString "Scanner stopped"))

(fn OnBarcodeScanned
  (params (ScannedCode :type String))
  (bind _output_get (Variables|Default|SetLastScannedCode ScannedCode))
  (Variables|Default|SetScannerStatus (Utilities|Text|ToText(String) (Utilities|String|Append "Code scanned: " _output_get))))